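; BP_BaseEnemy is a base enemy Blueprint that handles taking hits and dying.
; TakeHit, ignored once the enemy is dead, subtracts a fixed default damage from Health and updates IsAlive.
; A surviving enemy plays a hit reaction, while a fatal hit calls Death, which plays the death animation and disables mesh collision.
; The event graph and construction script contain no logic.
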(event EventBeginPlay)

(event Collision|EventActorBeginOverlap
  (params (OtherActor :type Actor%20Object%20Reference)))

(event EventTick
  (params (DeltaSeconds :type Float%20%28single-precision%29)))

(fn ConstructionScript)

(fn TakeHit
  (if (Variables|Default|GetIsAlive)
    (bind _output_get (Variables|Default|SetHealth (- (Variables|Default|GetHealth) (Variables|Default|GetDefaultDamage))))
    (bind _output_get_2 (Variables|Default|SetIsAlive (> _output_get 0.0)))
    (if _output_get_2
      (Components|Animation|PlayAnimation (Variables|Character|GetMesh) "/Game/AnimStarterPack/Hit_React_1.Hit_React_1" false)
      (else
        (CallFunction|Death)))))

(fn Death
  (bind _mesh (Variables|Character|GetMesh))
  (Components|Animation|PlayAnimation _mesh "/Game/AnimStarterPack/Death_1.Death_1" false)
  (Collision|SetCollisionEnabled _mesh "NoCollision"))